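; Actor component that gives its owner an on-screen name tag showing a name and HP.
; BeginPlay creates a BP_NameTagWidget with a reference back to the component and adds it to the viewport; EndPlay removes it.
; SetName and SetHP forward values to that widget.
; An unconnected chain would bind to the owner's BP_MonsterStatComponent to pull the monster's name, but never runs.
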(event `self.ReceiveBeginPlay`
  (bind _returnvalue (`|CreateWidget` "/Game/HackAndSlash/characters/BP_NameTagWidget.BP_NameTagWidget_C" null self))
  (bind _output_get (set `self.NameTag` _returnvalue))
  (`UserWidget.AddToViewport` _output_get 0))

(event `self.ReceiveEndPlay`
  (params (EndPlayReason :type "EEndPlayReason Enum" :default "Destroyed"))
  (`Widget.RemoveFromParent` (`self.NameTag`)))

(fn `BP_NameTagComponent_AutoGenFunc`
  (params (MonStat :type "/Game/HackAndSlash/Monster/ST_CurMonster Structure"))
  (locals (NewLocalVar :type "/Game/HackAndSlash/Monster/ST_Monster Structure"))
  (`/Game/HackAndSlash/characters/BP_NameTagWidget.SetName` (`self.NameTag`) (break `/Game/HackAndSlash/Monster/ST_Monster` (`.MonData_3_20C4B3E349683D2B5B787988D98BDFBE` (break `/Game/HackAndSlash/Monster/ST_CurMonster` MonStat)))))

(fn `SetHP`
  (params (CurHP :type "Float (double-precision)") (MaxHP :type "Float (double-precision)"))
  (`/Game/HackAndSlash/characters/BP_NameTagWidget.SetHP` (`self.NameTag`) CurHP MaxHP))

(fn `SetName`
  (params (name :type String))
  (`/Game/HackAndSlash/characters/BP_NameTagWidget.SetName` (`self.NameTag`) name))