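; Monster spawner component that spawns a random monster from DT_Monster around its owner every second.
; DoSpawn takes the class from a random row, spawns it with BT_Mon, then calls SetMonStat with a separately drawn random row name, so stats may mismatch the class.
; GetrandomcirleLocation offsets X and Y by cosine and sine of independent random angles scaled by Radius times pi, scattering within a square rather than on a circle.
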(event `self.ReceiveBeginPlay`
  (`KismetSystemLibrary.K2_SetTimer` null "DoSpawn" 1.0 true))

(fn `DoSpawn`
  (locals (NewLocalVar :type "Array of Name"))
  (bind _outrownames (`DataTableFunctionLibrary.GetDataTableRowNames` "/Game/HackAndSlash/Monster/DT_Monster.DT_Monster"))
  (bind _outitem (`KismetArrayLibrary.Array_Random` _outrownames))
  (bind _returnvalue (`|GetDataTableRow` "/Game/HackAndSlash/Monster/DT_Monster.DT_Monster" _outitem)
    (:`then`
      (bind _returnvalue_2 (`AIBlueprintHelperLibrary.SpawnAIFromClass` (`.MonsterClass_8_E9217B4743759A2CC343FBAFC1D3DCF5` (break `/Game/HackAndSlash/Monster/ST_Monster` _returnvalue)) "/Game/HackAndSlash/AI/BT_Mon.BT_Mon" (`self.GetrandomcirleLocation`) (struct) false null))
      (bind _asbp_monster_base (cast `/Game/HackAndSlash/Monster/BP_MonsterBase` _returnvalue_2))
      (`/Game/HackAndSlash/Monster/BP_MonsterBase.SetMonStat` _asbp_monster_base _outitem))))

(fn `GetrandomcirleLocation`
  (returns (ReturnValue :type "Vector Structure"))
  (locals (Rand :type "Float (double-precision)" :default 0.0))
  (bind _returnvalue (`KismetMathLibrary.RandomFloatInRange` 0.0 360.0))
  (bind _returnvalue_2 (* (`self.Radius`) 3.141592))
  (set `local.Rand` _returnvalue)
  (return (+ (`Actor.K2_GetActorLocation` (`self.GetOwner`)) (`KismetMathLibrary.MakeVector` (* (`KismetMathLibrary.Cos` _returnvalue) _returnvalue_2) (* (`KismetMathLibrary.Sin` _returnvalue) _returnvalue_2)))))