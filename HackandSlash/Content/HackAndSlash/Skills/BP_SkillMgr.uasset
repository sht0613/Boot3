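; BP_SkillMgr is a skill manager that automatically fires its owner's skills on cooldown.
; AddSkills looks up a DT_Skill row by name and stores it with its timer already at full cooldown, so it fires on the next update.
; Tick advances every timer; once one exceeds CoolTime, DoUseSkill spawns that SkillClass at the owner's transform, passing the owning Character, and the timer resets.
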(event `self.ReceiveTick`
  (params (DeltaSeconds :type "Float (single-precision)"))
  (`self.UpdateSkills` DeltaSeconds))

(fn `AddSkills`
  (params (RowName :type Name))
  ; 이 테이블에서 이 이름을 가진 데이터를 줘
  (bind _returnvalue (`|GetDataTableRow` "/Game/HackAndSlash/Skills/DT_Skill.DT_Skill" RowName)
    (:`then`
      (bind (_name _skillclass _cooltime) (break `/Game/HackAndSlash/Skills/ST_Skill` _returnvalue))
      (`KismetArrayLibrary.Array_Add` (`self.Skills`) (make `/Game/HackAndSlash/Skills/ST_CurSkill` _returnvalue _cooltime))
      (`KismetSystemLibrary.PrintString` (`KismetStringLibrary.Concat_StrStr` "AddSKill-" _name)))))

(fn `DoUseSkill`
  (params (CurSkill :type "/Game/HackAndSlash/Skills/ST_CurSkill Structure"))
  (bind _returnvalue (`self.GetOwner`))
  (`KismetSystemLibrary.PrintString` (`KismetStringLibrary.Concat_StrStr` "UseSkill2-" (break `/Game/HackAndSlash/Skills/ST_Skill` (`.Skilldata_4_A78F0A4F4C509EA21F1AA7BD0200F612` (break `/Game/HackAndSlash/Skills/ST_CurSkill` CurSkill)))))
  (bind _ascharacter (cast `Character` _returnvalue))
  (`|SpawnActorFromClass` (`.SkillClass_11_C7DB6FF1461336D8A62285A86A836802` (break `/Game/HackAndSlash/Skills/ST_Skill` (`.Skilldata_4_A78F0A4F4C509EA21F1AA7BD0200F612` (break `/Game/HackAndSlash/Skills/ST_CurSkill` CurSkill)))) (`Actor.GetTransform` _returnvalue) "Undefined" "MultiplyWithRoot" null _ascharacter null))

(fn `UpdateSkilCoolTime`
  (params (CurSkill :type "/Game/HackAndSlash/Skills/ST_CurSkill Structure (by ref)") (DeltaSec :type "Float (double-precision)"))
  (bind _structout (setmembers `/Game/HackAndSlash/Skills/ST_CurSkill` :`StructRef` CurSkill :`CurColltime` (+ (`.CurColltime_5_A8B922814B70AD05A3B4409D05A6044D` (break `/Game/HackAndSlash/Skills/ST_CurSkill` CurSkill)) DeltaSec)))
  (bind (_skilldata _curcolltime) (break `/Game/HackAndSlash/Skills/ST_CurSkill` _structout))
  (if (> _curcolltime (`.CoolTime_10_4D939CCF42F5D03F54AC3783173E28C7` (break `/Game/HackAndSlash/Skills/ST_Skill` _skilldata)))
    (`self.DoUseSkill` _structout)
    (setmembers `/Game/HackAndSlash/Skills/ST_CurSkill` :`StructRef` _structout :`CurColltime` 0.0)))

(fn `UpdateSkills`
  (params (DeltaSec :type "Float (double-precision)"))
  (for (_ _array_index) (`self.Skills`)
    (`self.UpdateSkilCoolTime` (`|GetArrayItem` (`self.Skills`) _array_index) DeltaSec)))